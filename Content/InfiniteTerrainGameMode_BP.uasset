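; Game mode for an infinite-terrain game that spawns the opening run of tiles and tracks the score.
; BeginPlay fills a NavMesh bounds volume pool, then calls SpawnTile repeatedly.
; Each spawned Tile_BP receives the shared pool, and its attach location becomes the next tile's transform, chaining tiles together.
; NewTailConquered increments the score and prints it.
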(event `self.ReceiveBeginPlay`
  (`self.PopulateBoundsVolumePool`)
  (for _ (range 3)
    (`self.SpawnTile`)))

(event `self.ReceiveTick`
  (params (DeltaSeconds :type "Float (single-precision)")))

(fn `NewTailConquered`
  (bind _result (`/Engine/EditorBlueprintResources/StandardMacros.IncrementInt` (`self.Score`))
    (:`  `
      (`KismetSystemLibrary.PrintString` (`KismetStringLibrary.Conv_IntToString` _result)))))

(fn `SpawnTile`
  (bind _returnvalue (`|SpawnActorFromClass` "/Game/Terrain/Tile_BP.Tile_BP_C" (`self.NextTileTransform`) "Undefined" "OverrideRootScale" null null))
  (`Tile.SetPool` _returnvalue (`self.NavMeshBoundsVolumePool`))
  (bind _attachtransform (`/Game/Terrain/Tile_BP.GetAttachLocation` _returnvalue))
  (set `self.NextTileTransform` _attachtransform))

(fn `UserConstructionScript`)